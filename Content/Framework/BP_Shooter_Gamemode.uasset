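; Shooter game mode that gathers joining player controllers, spawns their chosen characters and starts the match.
; It waits for the player count from the game instance, or starts at once in solo, then restarts each player at an index-named start.
; After a countdown it enables all input.
; The pawn spawn override reads class, model and skin from PlayerState under seamless travel, otherwise from the controller.
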(event Custom|LevelStart
  (Utilities|FlowControl|Delay 0.2)
  (for _array_element (Variables|Default|GetAllConnectedControllers)
    (Default|GameStartCountdown _array_element))
  (Utilities|FlowControl|Delay 3.0)
  (for _array_element_2 (Variables|Default|GetAllConnectedControllers)
    (Default|EnableAllInput _array_element_2)))

(event EventOnLogout
  (params (ExitingController :type Controller%20Object%20Reference))
  (bind _asbp_shooter_player_controller (Utilities|Casting|CastToBP_Shooter_PlayerController ExitingController))
  (Utilities|Array|RemoveItem (Variables|Default|GetAllConnectedControllers) _asbp_shooter_player_controller)
  (Math|Integer|DecrementInt (Variables|Default|Getnum_ExpectedPlayers)))

(event EventBeginPlay
  (bind _asbp_shooter_game_instance (Utilities|Casting|CastToBP_Shooter_GameInstance (Game|GetGameInstance)))
  (Variables|Default|SetbUseSeamlessTravel (Variables|/Game/Framework/BP_Shooter_GameInstance.BP_Shooter_GameInstance_C|GetSeamlessTravelEnabled _asbp_shooter_game_instance))
  (Variables|Default|SetSeamless%20Travel%20Enabled (Variables|/Game/Framework/BP_Shooter_GameInstance.BP_Shooter_GameInstance_C|GetSeamlessTravelEnabled _asbp_shooter_game_instance)))

(event EventHandleStartingNewPlayer
  (params (NewPlayer :type Player%20Controller%20Object%20Reference))
  (bind _asbp_shooter_player_controller (Utilities|Casting|CastToBP_Shooter_PlayerController NewPlayer))
  (Utilities|Array|Add (Variables|Default|GetAllConnectedControllers) _asbp_shooter_player_controller)
  (bind _asbp_shooter_game_instance (Utilities|Casting|CastToBP_Shooter_GameInstance (Game|GetGameInstance)))
  (Variables|Default|Setnum_ExpectedPlayers (Variables|/Game/Framework/BP_Shooter_GameInstance.BP_Shooter_GameInstance_C|GetNumConnectedPlayers _asbp_shooter_game_instance))
  (if (Variables|/Game/Framework/BP_Shooter_GameInstance.BP_Shooter_GameInstance_C|GetIsSoloGame _asbp_shooter_game_instance)
    (Variables|Default|Setnum_ExpectedPlayers 1)
    (Class|GameModeBase|RestartPlayeratPlayerStart (Utilities|Array|Get(acopy) (Variables|Default|GetAllConnectedControllers)) (Class|GameModeBase|FindPlayerStart 0 "0"))
    (CallFunction|LevelStart)
    (elif (== (Variables|Default|Getnum_ExpectedPlayers) (Utilities|Array|Length (Variables|Default|GetAllConnectedControllers)))
      (Utilities|FlowControl|Delay 0.5)
      (for (_array_element _array_index) (Variables|Default|GetAllConnectedControllers)
        (Class|GameModeBase|RestartPlayeratPlayerStart _array_element (Class|GameModeBase|FindPlayerStart _array_element (Utilities|String|ToString(Integer) _array_index))))
      (CallFunction|LevelStart))))

(fn ConstructionScript)

(fn SpawnDefaultPawnfor
  (params (NewPlayer :type Controller%20Object%20Reference) (StartSpot :type Actor%20Object%20Reference))
  (if (Variables|Default|GetSeamless%20Travel%20Enabled)
    (bind _asbp_shooter_player_state (Utilities|Casting|CastToBP_Shooter_PlayerState (Variables|/Script/Engine.Controller|GetPlayerState NewPlayer)))
    (LocalVariables|SetLocal_CharacterClass (.characterclass (Variables|/Game/Framework/BP_Shooter_PlayerState.BP_Shooter_PlayerState_C|GetS_PlayerProfile _asbp_shooter_player_state)))
    (LocalVariables|SetLocal_ModelName (.modelname (Variables|/Game/Framework/BP_Shooter_PlayerState.BP_Shooter_PlayerState_C|GetS_PlayerProfile _asbp_shooter_player_state)))
    (LocalVariables|SetLocal_SkinName (.skinname (Variables|/Game/Framework/BP_Shooter_PlayerState.BP_Shooter_PlayerState_C|GetS_PlayerProfile _asbp_shooter_player_state)))
    (else
      (bind _asbp_shooter_player_controller (Utilities|Casting|CastToBP_Shooter_PlayerController NewPlayer))
      (LocalVariables|SetLocal_CharacterClass (.CharacterClass (Utilities|Struct|BreakS_PlayerProfile (Variables|/Game/Framework/BP_Shooter_PlayerController.BP_Shooter_PlayerController_C|GetPlayer%20Profile%20Struct _asbp_shooter_player_controller))))
      (LocalVariables|SetLocal_ModelName (.ModelName (Utilities|Struct|BreakS_PlayerProfile (Variables|/Game/Framework/BP_Shooter_PlayerController.BP_Shooter_PlayerController_C|GetPlayer%20Profile%20Struct _asbp_shooter_player_controller))))
      (LocalVariables|SetLocal_SkinName (.SkinName (Utilities|Struct|BreakS_PlayerProfile (Variables|/Game/Framework/BP_Shooter_PlayerController.BP_Shooter_PlayerController_C|GetPlayer%20Profile%20Struct _asbp_shooter_player_controller))))))
  (bind _returnvalue (Game|SpawnActorfromClass (LocalVariables|GetLocal_CharacterClass) (Transformation|GetActorTransform StartSpot) "Undefined" 0 0))
  (bind _asbp_shooter_player_base (Utilities|Casting|CastToBP_ShooterPlayer_Base _returnvalue))
  (Variables|/Game/Blueprints/Player/BP_ShooterPlayer_Base.BP_ShooterPlayer_Base_C|SetModelName _asbp_shooter_player_base (LocalVariables|GetLocal_ModelName))
  (Variables|/Game/Blueprints/Player/BP_ShooterPlayer_Base.BP_ShooterPlayer_Base_C|SetSkinName _asbp_shooter_player_base (LocalVariables|GetLocal_SkinName))
  (return _asbp_shooter_player_base))