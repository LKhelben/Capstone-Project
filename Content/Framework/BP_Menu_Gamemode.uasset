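; Menu game mode that runs the multiplayer lobby, tracking connected controllers and their profiles.
; Joining players on the lobby map get a menu; logout destroys their character and frees its spot.
; Updates copy profiles into player states, push names and level selection to controllers, and spawn characters at free spots.
; Meshes, animations and skins come from a customization data table, applied through multicast calls, or client calls for previews.
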(event Custom|UpdateLobbyEvent
  (params (PlayerNames :type Boolean) (LevelSelection :type Boolean) (CharacterSelection :type Boolean))
  (Utilities|Array|Clear (Variables|Default|GetAll_PlayerProfiles))
  (for (_array_element _array_index) (Variables|Default|GetAll_ConnectedPlayers)
    (Utilities|Array|SetArrayElem (Variables|Default|GetAll_PlayerProfiles) _array_index (Variables|/Game/Framework/BP_Menu_Controller.BP_Menu_Controller_C|GetPlayerProfileInfo _array_element) true)
    (bind _asbp_shooter_player_state (Utilities|Casting|CastToBP_Shooter_PlayerState (Variables|/Script/Engine.Controller|GetPlayerState _array_element)))
    (Variables|/Game/Framework/BP_Shooter_PlayerState.BP_Shooter_PlayerState_C|SetS_PlayerProfile _asbp_shooter_player_state (Variables|/Game/Framework/BP_Menu_Controller.BP_Menu_Controller_C|GetPlayerProfileInfo _array_element)))
  (for (_array_element_2 _array_index_2) (Variables|Default|GetAll_ConnectedPlayers)
    (if PlayerNames
      (Default|UpdatePlayerNames _array_element_2 (Variables|Default|GetAll_PlayerProfiles)))
    (if LevelSelection
      (Default|UpdateLevelSelection _array_element_2 (Variables|Default|GetSelectedLevelName)))
    (if CharacterSelection
      (CallFunction|UpdateSelectedCharacter _array_index_2))))

(event Custom|UpdateSelectedCharacter
  (params (PlayerIndex :type Integer))
  (bind _all_connectedplayers (Variables|Default|GetAll_ConnectedPlayers))
  (bind _all_connectedplayers_2 (Variables|Default|GetAll_ConnectedPlayers))
  (bind _all_playerprofiles (Variables|Default|GetAll_PlayerProfiles))
  (bind _output (Utilities|Array|Get(acopy) _all_connectedplayers PlayerIndex))
  (bind _output_2 (Utilities|Array|Get(acopy) _all_connectedplayers_2 PlayerIndex))
  (bind _output_3 (Utilities|Array|Get(acopy) _all_playerprofiles PlayerIndex))
  (if (== (Variables|/Game/Framework/BP_Menu_Controller.BP_Menu_Controller_C|GetLobbyCharacter _output) 0)
    (bind _availableplayerspot (CallFunction|GetLobbyPlayerSpot))
    (Variables|/Game/Gameplay/Lobby/BP_Lobby_PlayerSpot.BP_Lobby_PlayerSpot_C|SetIsSpotUsed _availableplayerspot true)
    (bind _returnvalue (Game|SpawnActorfromClass "/Game/Gameplay/Lobby/BP_Lobby_Character.BP_Lobby_Character_C" (Transformation|GetActorTransform _availableplayerspot) "Undefined" _output 0))
    (Variables|/Game/Framework/BP_Menu_Controller.BP_Menu_Controller_C|SetLobbyCharacter _output_2 _returnvalue)
    (Variables|/Game/Framework/BP_Menu_Controller.BP_Menu_Controller_C|SetLobbyPlayerSpot _output_2 _availableplayerspot))
  (Default|MCSetPlayerName (Variables|/Game/Framework/BP_Menu_Controller.BP_Menu_Controller_C|GetLobbyCharacter (Utilities|Array|Get(acopy) (Variables|Default|GetAll_ConnectedPlayers) PlayerIndex)) (.playername _output_3))
  (bind _returnvalue_2 (Utilities|GetDataTableRow "/Game/Blueprints/Player/Structures_and_Tables/CharacterCustomization_Table.CharacterCustomization_Table" (.characterrowname _output_3))
    (:then
      (Default|MCSetCharacterMesh (Variables|/Game/Framework/BP_Menu_Controller.BP_Menu_Controller_C|GetLobbyCharacter (Utilities|Array|Get(acopy) (Variables|Default|GetAll_ConnectedPlayers) PlayerIndex)) (.Model (Utilities|Struct|BreakS_ModelAndSkins (.Value (Utilities|Map|Find (.ModelsAndSkins (Utilities|Struct|BreakS_CharacterCustomization _returnvalue_2)) (.modelname _output_3))))))
      (Default|MCPlayMeshAnimation (Variables|/Game/Framework/BP_Menu_Controller.BP_Menu_Controller_C|GetLobbyCharacter (Utilities|Array|Get(acopy) (Variables|Default|GetAll_ConnectedPlayers) PlayerIndex)) (.LobbyAnimation (Utilities|Struct|BreakS_ModelAndSkins (.Value (Utilities|Map|Find (.ModelsAndSkins (Utilities|Struct|BreakS_CharacterCustomization _returnvalue_2)) (.modelname _output_3))))))
      (if (.Use_Skin0 (Utilities|Struct|BreakS_ModelAndSkins (.Value (Utilities|Map|Find (.ModelsAndSkins (Utilities|Struct|BreakS_CharacterCustomization _returnvalue_2)) (.modelname _output_3)))))
        (Default|MCSetSkinMaterial (Variables|/Game/Framework/BP_Menu_Controller.BP_Menu_Controller_C|GetLobbyCharacter (Utilities|Array|Get(acopy) (Variables|Default|GetAll_ConnectedPlayers) PlayerIndex)) (.Skin0_MaterialSlot (Utilities|Struct|BreakS_ModelAndSkins (.Value (Utilities|Map|Find (.ModelsAndSkins (Utilities|Struct|BreakS_CharacterCustomization _returnvalue_2)) (.modelname _output_3))))) (.Value (Utilities|Map|Find (.Skin0_Skins (Utilities|Struct|BreakS_ModelAndSkins (.Value (Utilities|Map|Find (.ModelsAndSkins (Utilities|Struct|BreakS_CharacterCustomization _returnvalue_2)) (.modelname _output_3))))) (.skinname _output_3)))))
      (if (.Use_Skin1 (Utilities|Struct|BreakS_ModelAndSkins (.Value (Utilities|Map|Find (.ModelsAndSkins (Utilities|Struct|BreakS_CharacterCustomization _returnvalue_2)) (.modelname _output_3)))))
        (Default|MCSetSkinMaterial (Variables|/Game/Framework/BP_Menu_Controller.BP_Menu_Controller_C|GetLobbyCharacter (Utilities|Array|Get(acopy) (Variables|Default|GetAll_ConnectedPlayers) PlayerIndex)) (.Skin1_MaterialSlot (Utilities|Struct|BreakS_ModelAndSkins (.Value (Utilities|Map|Find (.ModelsAndSkins (Utilities|Struct|BreakS_CharacterCustomization _returnvalue_2)) (.modelname _output_3))))) (.Value (Utilities|Map|Find (.Skin1_Skins (Utilities|Struct|BreakS_ModelAndSkins (.Value (Utilities|Map|Find (.ModelsAndSkins (Utilities|Struct|BreakS_CharacterCustomization _returnvalue_2)) (.modelname _output_3))))) (.skinname _output_3))))))))

(event Custom|UpdateCharacterForController
  (params (PlayerController :type BP%20Menu%20Controller%20Object%20Reference) (PlayerProfile :type S%20Player%20Profile%20Structure))
  (bind _all_connectedplayers (Variables|Default|GetAll_ConnectedPlayers))
  (bind _returnvalue (Utilities|Array|FindItem _all_connectedplayers PlayerController))
  (Utilities|Array|SetArrayElem (Variables|Default|GetAll_PlayerProfiles) _returnvalue PlayerProfile true)
  (bind _asbp_shooter_player_state (Utilities|Casting|CastToBP_Shooter_PlayerState (Variables|/Script/Engine.Controller|GetPlayerState PlayerController)))
  (Variables|/Game/Framework/BP_Shooter_PlayerState.BP_Shooter_PlayerState_C|SetS_PlayerProfile _asbp_shooter_player_state PlayerProfile)
  (CallFunction|UpdateSelectedCharacter _returnvalue))

(event Custom|PreviewCharacterForController
  (params (Controller :type BP%20Menu%20Controller%20Object%20Reference) (CharacterRowName :type Name) (ModelName :type Name) (SkinName :type Name))
  (bind _lobbycharacter (Variables|/Game/Framework/BP_Menu_Controller.BP_Menu_Controller_C|GetLobbyCharacter Controller))
  (bind _returnvalue (Utilities|GetDataTableRow "/Game/Blueprints/Player/Structures_and_Tables/CharacterCustomization_Table.CharacterCustomization_Table" CharacterRowName)
    (:then
      (Default|ClientSetCharacterMesh _lobbycharacter (.Model (Utilities|Struct|BreakS_ModelAndSkins (.Value (Utilities|Map|Find (.ModelsAndSkins (Utilities|Struct|BreakS_CharacterCustomization _returnvalue)) ModelName)))))
      (Default|ClientPlayMeshAnimation _lobbycharacter (.LobbyAnimation (Utilities|Struct|BreakS_ModelAndSkins (.Value (Utilities|Map|Find (.ModelsAndSkins (Utilities|Struct|BreakS_CharacterCustomization _returnvalue)) ModelName)))))
      (if (.Use_Skin0 (Utilities|Struct|BreakS_ModelAndSkins (.Value (Utilities|Map|Find (.ModelsAndSkins (Utilities|Struct|BreakS_CharacterCustomization _returnvalue)) ModelName))))
        (Default|ClientSetSkinMaterial _lobbycharacter (.Skin0_MaterialSlot (Utilities|Struct|BreakS_ModelAndSkins (.Value (Utilities|Map|Find (.ModelsAndSkins (Utilities|Struct|BreakS_CharacterCustomization _returnvalue)) ModelName)))) (.Value (Utilities|Map|Find (.Skin0_Skins (Utilities|Struct|BreakS_ModelAndSkins (.Value (Utilities|Map|Find (.ModelsAndSkins (Utilities|Struct|BreakS_CharacterCustomization _returnvalue)) ModelName)))) SkinName))))
      (if (.Use_Skin1 (Utilities|Struct|BreakS_ModelAndSkins (.Value (Utilities|Map|Find (.ModelsAndSkins (Utilities|Struct|BreakS_CharacterCustomization _returnvalue)) ModelName))))
        (Default|ClientSetSkinMaterial _lobbycharacter (.Skin1_MaterialSlot (Utilities|Struct|BreakS_ModelAndSkins (.Value (Utilities|Map|Find (.ModelsAndSkins (Utilities|Struct|BreakS_CharacterCustomization _returnvalue)) ModelName)))) (.Value (Utilities|Map|Find (.Skin1_Skins (Utilities|Struct|BreakS_ModelAndSkins (.Value (Utilities|Map|Find (.ModelsAndSkins (Utilities|Struct|BreakS_CharacterCustomization _returnvalue)) ModelName)))) SkinName)))))))

(event EventHandleStartingNewPlayer
  (params (NewPlayer :type Player%20Controller%20Object%20Reference))
  (bind _returnvalue (Game|GetCurrentLevelName true))
  (switch string _returnvalue
    (:LobbyMenu_Map
      (bind _asbp_menu_controller (Utilities|Casting|CastToBP_Menu_Controller NewPlayer))
      (Utilities|Array|Add (Variables|Default|GetAll_ConnectedPlayers) _asbp_menu_controller)
      (Default|CreateLobbyMenu _asbp_menu_controller)
      (Default|InitialSetup _asbp_menu_controller))))

(event EventOnLogout
  (params (ExitingController :type Controller%20Object%20Reference))
  (bind _asbp_menu_controller (Utilities|Casting|CastToBP_Menu_Controller ExitingController))
  (if (== (Variables|/Game/Framework/BP_Menu_Controller.BP_Menu_Controller_C|GetLobbyCharacter _asbp_menu_controller) 0)
    _
    (else
      (Actor|DestroyActor (Variables|/Game/Framework/BP_Menu_Controller.BP_Menu_Controller_C|GetLobbyCharacter _asbp_menu_controller))
      (Variables|/Game/Gameplay/Lobby/BP_Lobby_PlayerSpot.BP_Lobby_PlayerSpot_C|SetIsSpotUsed (Variables|/Game/Framework/BP_Menu_Controller.BP_Menu_Controller_C|GetLobbyPlayerSpot _asbp_menu_controller) false)))
  (Utilities|Array|RemoveItem (Variables|Default|GetAll_ConnectedPlayers) _asbp_menu_controller)
  (CallFunction|UpdateLobbyEvent true false true))

(fn ConstructionScript)

(fn GetLobbyPlayerSpot
  (if (== (Utilities|Array|Length (Variables|Default|GetAll_LobbyPlayerSpotsArray)) 0)
    (bind _outactors (Actor|GetAllActorsOfClass "/Game/Gameplay/Lobby/BP_Lobby_PlayerSpot.BP_Lobby_PlayerSpot_C"))
    (Variables|Default|SetAll_LobbyPlayerSpotsArray _outactors))
  (bind _array_element (Utilities|Array|ForEachLoopwithBreak (Variables|Default|GetAll_LobbyPlayerSpotsArray) :!label _label)
    (:LoopBody
      (if (not (Variables|/Game/Gameplay/Lobby/BP_Lobby_PlayerSpot.BP_Lobby_PlayerSpot_C|GetIsSpotUsed _array_element))
        (goto _label Break)))
    (:Completed
      (return _array_element))))