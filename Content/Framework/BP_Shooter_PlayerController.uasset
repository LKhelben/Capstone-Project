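; Player controller for the shooter that sets up the in-game HUD and loads and saves the player's profile.
; On local BeginPlay it creates the HUD and loads the profile save, setting it directly with authority or sending it to the server otherwise.
; On possess it hands the HUD reference to the pawn, and XP/level saves are debounced with a retriggerable delay.
; Other events handle countdown, HUD visibility, input enabling and leaving the session for the main menu.
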(event Custom|EnableAllInput
  (Input|EnableInput (Pawn|GetControlledPawn) self))

(event Custom|GameStartCountdown
  (Default|GameStartCountdown (Variables|Default|GetWD_InGamePlayerHUDRef)))

(event Custom|UnhideInGameHUD
  (Widget|SetVisibility (Variables|Default|GetWD_InGamePlayerHUDRef) "Visible"))

(event Custom|EndClientSession
  (bind _asbp_shooter_game_instance (Utilities|Casting|CastToBP_Shooter_GameInstance (Game|GetGameInstance)))
  (Variables|/Game/Framework/BP_Shooter_GameInstance.BP_Shooter_GameInstance_C|SetMP_IsPauseMenuVisible _asbp_shooter_game_instance false)
  (|DestroySession self
    (:then
      (Game|OpenLevel(byName) "MainMenu_Map"))))

(event Custom|Local_SetHUDVariable
  (bind _asbp_shooter_player_base (Utilities|Casting|CastToBP_ShooterPlayer_Base (Pawn|GetControlledPawn)))
  (Variables|/Game/Blueprints/Player/BP_ShooterPlayer_Base.BP_ShooterPlayer_Base_C|SetWD%20in%20Game%20Player%20HUDRef _asbp_shooter_player_base (Variables|Default|GetWD_InGamePlayerHUDRef)))

(event Custom|Server_SetPlayerProfile
  (params (Player%20Profile%20Struct :type S%20Player%20Profile%20Structure))
  (Variables|Default|SetPlayer%20Profile%20Struct Player%20Profile%20Struct))

(event Custom|Save_XPandLevel
  (bind _as_sg_player_profile (Variables|Default|GetAs%20SG%20Player%20Profile))
  (Utilities|FlowControl|RetriggerableDelay 0.5)
  (Variables|/Game/Framework/SavedData/SG_PlayerProfile.SG_PlayerProfile_C|SetPlayerProfileStruct _as_sg_player_profile (Variables|Default|GetPlayer%20Profile%20Struct))
  (SaveGame|SaveGametoSlot _as_sg_player_profile "PlayerProfile_Slot"))

(event EventBeginPlay
  (if (Pawn|IsLocalPlayerController)
    (Viewport|RemoveAllWidgets)
    (CallFunction|UIShowinGameHUD)
    (Input|SetInputModeGameOnly self false)
    (Variables|Default|SetbShowMouseCursor false)
    (bind _returnvalue (SaveGame|LoadGamefromSlot "PlayerProfile_Slot"))
    (bind _assg_player_profile (Utilities|Casting|CastToSG_PlayerProfile _returnvalue))
    (Variables|Default|SetAs%20SG%20Player%20Profile _assg_player_profile)
    (Networking|SwitchHasAuthority
      (:Authority
        (Variables|Default|SetPlayer%20Profile%20Struct (Variables|/Game/Framework/SavedData/SG_PlayerProfile.SG_PlayerProfile_C|GetPlayerProfileStruct _assg_player_profile)))
      (:Remote
        (CallFunction|ServerSetPlayerProfile (Variables|/Game/Framework/SavedData/SG_PlayerProfile.SG_PlayerProfile_C|GetPlayerProfileStruct _assg_player_profile))))))

(event EventPossess
  (params (PossessedPawn :type Pawn%20Object%20Reference))
  (CallFunction|LocalSetHUDVariable))

(fn ConstructionScript)

(fn UIShowinGameHUD
  (Utilities|IsValid (Variables|Default|GetWD_InGamePlayerHUDRef)
    (:Is%20Valid
      _)
    (:Is%20Not%20Valid
      (bind _returnvalue (UserInterface|CreateWidget "/Game/Widgets/Player_Widgets/WD_PlayerInGameHUD.WD_PlayerInGameHUD_C" self))
      (Variables|Default|SetWD_InGamePlayerHUDRef _returnvalue)))
  (UserInterface|Viewport|AddtoViewport (Variables|Default|GetWD_InGamePlayerHUDRef) 0)
  (return))