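; BP_Lobby_Character is the lobby's display character, showing a player's name, skeletal mesh, skin material and looping animation.
; Paired MC_ and Client_ events, named as multicast and client-targeted variants, apply the same mesh, animation and material changes to CharacterMesh.
; The name has only an MC_ event, which calls SetPlayerName to set the PlayerName text.
; The Blueprint holds no selection logic, so callers supply every value.
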(event Custom|MC_PlayMeshAnimation
  (params (NewAnimToPlay :type Animation%20Asset%20Object%20Reference))
  (Components|Animation|PlayAnimation (Variables|Default|GetCharacterMesh) NewAnimToPlay true))

(event Custom|MC_SetSkinMaterial
  (params (ElementIndex :type Integer) (Material :type Material%20Interface%20Object%20Reference))
  (Rendering|Material|SetMaterial (Variables|Default|GetCharacterMesh) ElementIndex Material))

(event Custom|Client_SetCharacterMesh
  (params (NewMesh :type Skeletal%20Mesh%20Object%20Reference))
  (Components|SkeletalMesh|SetSkeletalMeshAsset (Variables|Default|GetCharacterMesh) NewMesh))

(event Custom|Client_PlayMeshAnimation
  (params (NewAnimToPlay :type Animation%20Asset%20Object%20Reference))
  (Components|Animation|PlayAnimation (Variables|Default|GetCharacterMesh) NewAnimToPlay true))

(event Custom|Client_SetSkinMaterial
  (params (ElementIndex :type Integer) (Material :type Material%20Interface%20Object%20Reference))
  (Rendering|Material|SetMaterial (Variables|Default|GetCharacterMesh) ElementIndex Material))

(event Custom|MC_SetPlayerName
  (params (TextValuePlayerName :type Text))
  (CallFunction|SetPlayerName TextValuePlayerName))

(event Custom|MC_SetCharacterMesh
  (params (NewMesh :type Skeletal%20Mesh%20Object%20Reference))
  (Components|SkeletalMesh|SetSkeletalMeshAsset (Variables|Default|GetCharacterMesh) NewMesh))

(fn ConstructionScript)

(fn SetPlayerName
  (params (TextValuePlayerName :type Text))
  (Rendering|Components|TextRender|SetText (Variables|Default|GetPlayerName) TextValuePlayerName))