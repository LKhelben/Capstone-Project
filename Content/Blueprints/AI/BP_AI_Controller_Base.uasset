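; Base AI controller for grunt enemies that uses sight perception to pick and chase players.
; On possess it caches the controlled BP_AI_Grunt_Base.
; When sight detects a new shooter player and target switching is allowed, it locks switching, sets that player as the grunt's enemy and tells it to move to them.
; Seeing the current target keeps the lock, while losing sight of it allows switching again.
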(event OnTargetPerceptionUpdated(AIPerception)
  (params (Actor :type Actor%20Object%20Reference) (Stimulus :type AI%20Stimulus%20Structure))
  (bind _bsuccessfullysensed (Utilities|Struct|BreakAIStimulus Stimulus))
  (bind _gruntbase_ref (Variables|Default|GetGruntBase_Ref))
  ;[1 1 1] AI Sight Perception Finding New Players
  (bind _returnvalue (Class|AIPerceptionSystem|GetSenseClassforStimulus Stimulus))
  (if (== _returnvalue "/Script/AIModule.AISense_Sight")
    (if (!= Actor (Variables|Default|GetTargetPlayer))
      (bind _asbp_shooter_player_base (Utilities|Casting|CastToBP_ShooterPlayer_Base Actor))
      (if _bsuccessfullysensed
        (if (Variables|Default|GetCanSwitchTargets)
          (Variables|Default|SetCanSwitchTargets false)
          (Default|SetTargetPlayerEnemy _gruntbase_ref _asbp_shooter_player_base)
          (Default|MovetoPlayer _gruntbase_ref)))
      (elif _bsuccessfullysensed
        (Variables|Default|SetCanSwitchTargets false)
        (else
          (Variables|Default|SetCanSwitchTargets true))))))

(event EventPossess
  (params (PossessedPawn :type Pawn%20Object%20Reference))
  (bind _asbp_ai_grunt_base (Utilities|Casting|CastToBP_AI_Grunt_Base PossessedPawn))
  (Variables|Default|SetGruntBase_Ref _asbp_ai_grunt_base))

(fn ConstructionScript)