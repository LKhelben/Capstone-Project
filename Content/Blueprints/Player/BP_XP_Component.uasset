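; Player component that tracks XP and level for the shooter player character.
; On initialize it copies an XP-per-level threshold map and loads current values from the first player controller's profile struct.
; Adding XP scans thresholds up to the level cap, allowing multi-level jumps, then writes back to that profile.
; For the local player, it refreshes the HUD, saves progress and plays a level-up animation when earned.
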(event Custom|XP_Component_Initialize
  (CallFunction|SetupXpMap)
  (bind _asbp_shooter_player_base (Utilities|Casting|CastToBP_ShooterPlayer_Base (Components|GetOwner)))
  (Variables|Default|SetShooter%20Player%20Base _asbp_shooter_player_base)
  (bind _asbp_shooter_player_controller (Utilities|Casting|CastToBP_Shooter_PlayerController (Game|GetPlayerController 0)))
  (bind _output_get (Variables|Default|SetShooter%20Player%20Controller _asbp_shooter_player_controller))
  (Variables|Default|SetPlayer%20XP (.playerxp (Variables|/Game/Framework/BP_Shooter_PlayerController.BP_Shooter_PlayerController_C|GetPlayer%20Profile%20Struct _output_get)))
  (Variables|Default|SetPlayer%20Level (.playerlevel (Variables|/Game/Framework/BP_Shooter_PlayerController.BP_Shooter_PlayerController_C|GetPlayer%20Profile%20Struct _output_get)))
  (if (Pawn|IsLocalPlayerController (Variables|Default|GetShooter%20Player%20Controller))
    (Default|UpdateXPAmount (Variables|/Game/Framework/BP_Shooter_PlayerController.BP_Shooter_PlayerController_C|GetWD_InGamePlayerHUDRef (Variables|Default|GetShooter%20Player%20Controller)))
    (Default|UpdateLevelAmount (Variables|/Game/Framework/BP_Shooter_PlayerController.BP_Shooter_PlayerController_C|GetWD_InGamePlayerHUDRef (Variables|Default|GetShooter%20Player%20Controller)))
    (Default|SaveXPandLevel (Variables|Default|GetShooter%20Player%20Controller))))

(event Custom|Component_Add_XP
  (params (XP%20Amount :type Integer))
  (bind _shooter_player_base (Variables|Default|GetShooter%20Player%20Base))
  (bind _shooter_player_controller (Variables|Default|GetShooter%20Player%20Controller))
  (bind _wd_in_game_player_hudref (Variables|/Game/Blueprints/Player/BP_ShooterPlayer_Base.BP_ShooterPlayer_Base_C|GetWD%20in%20Game%20Player%20HUDRef _shooter_player_base))
  (bind _output_get (Variables|Default|SetPlayer%20XP (+ (Variables|Default|GetPlayer%20XP) XP%20Amount)))
  (bind (_canlevelup _newlevel) (CallFunction|CheckforLevelUp _output_get))
  (if _canlevelup
    (Variables|Default|SetPlayer%20Level _newlevel))
  (CallFunction|UpdatePlayerControllerProfile)
  (if (Pawn|IsLocallyControlled _shooter_player_base)
    (Default|UpdateXPAmount _wd_in_game_player_hudref)
    (Default|UpdateLevelAmount _wd_in_game_player_hudref)
    (Default|SaveXPandLevel _shooter_player_controller)
    (if _canlevelup
      (Default|PlayUIAnimLevelUp (Variables|/Game/Framework/BP_Shooter_PlayerController.BP_Shooter_PlayerController_C|GetWD_InGamePlayerHUDRef _shooter_player_controller)))))

(fn SetupXpMap
  (Variables|Default|SetXP%20Map%20Levels (.xp_maps_levels (LocalVariables|GetS_XPandLevel)))
  (return))

(fn CheckforLevelUp
  (params (XPAmount :type Integer))
  (LocalVariables|SetLocal_CurrentPlayerXP XPAmount)
  (LocalVariables|SetLocal_PlayerLevel (Variables|Default|GetPlayer%20Level))
  (if (and (> (LocalVariables|GetLocal_CurrentPlayerXP) (Utilities|Array|Get(acopy) (Variables|Default|GetXP%20Map%20Levels) (LocalVariables|GetLocal_PlayerLevel))) (< (LocalVariables|GetLocal_PlayerLevel) (Variables|Default|GetLevelMaxCap)))
    (LocalVariables|SetLocal_CanLevelUp true)
    (bind _index (Utilities|FlowControl|ForLoopwithBreak (LocalVariables|GetLocal_PlayerLevel) (Variables|Default|GetLevelMaxCap) :!label _label)
      (:LoopBody
        (if (not (> (LocalVariables|GetLocal_CurrentPlayerXP) (Utilities|Array|Get(acopy) (Variables|Default|GetXP%20Map%20Levels) _index)))
          (LocalVariables|SetLocal_PlayerLevel _index)
          (goto _label Break)))
      (:Completed
        (return (LocalVariables|GetLocal_CanLevelUp) (LocalVariables|GetLocal_PlayerLevel))))
    (else
      (LocalVariables|SetLocal_CanLevelUp false)
      (return (LocalVariables|GetLocal_CanLevelUp) (LocalVariables|GetLocal_PlayerLevel)))))

(fn UpdatePlayerControllerProfile
  (Utilities|Struct|SetmembersinS_PlayerProfile (Variables|/Game/Framework/BP_Shooter_PlayerController.BP_Shooter_PlayerController_C|GetPlayer%20Profile%20Struct (Variables|Default|GetShooter%20Player%20Controller)) (Variables|Default|GetPlayer%20XP) (Variables|Default|GetPlayer%20Level))
  (return))